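; BP_cachette is a hiding spot, a barrel judging by its sounds, with its own look input and a prompt text shown while something overlaps its collision.
; Interact hides the player actor, sets the BP_personnage Hidden variable to false and plays the barrel-in sound.
; The Action input finds every BP_personnage, possesses and unhides each in turn, and plays the barrel-out sound.
; Possession of the hiding spot itself is not handled in this Blueprint.
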(event `InputAxis|Turn`
  (params (AxisValue :type "Float (single-precision)"))
  ;[1 1 1] Caméra
  (`self.AddControllerYawInput` AxisValue))

(event `InputAxis|LookUp`
  (params (AxisValue :type "Float (single-precision)"))
  ;[1 1 1] Caméra
  (`self.AddControllerPitchInput` AxisValue))

(event `/Game/Personnage/BPI_hideout.Interact`
  (params (Player :type "Pawn Object Reference"))
  ;[1 1 1] Interaction
  (`self.SetActorHiddenInGame` Player true)
  (bind _asbp_personnage (cast `/Game/Personnage/BP_personnage` Player))
  (set `/Game/Personnage/BP_personnage.Hidden` false _asbp_personnage)
  ;[1 1 1] Sound Barrel In
  (`FMODAudioComponent.Play` (`self.SND_BarrelIn`)))

(event `self.Collision.OnComponentBeginOverlap`
  (params (OverlappedComponent :type "PrimitiveComponent Object Reference") (OtherActor :type "Actor Object Reference") (OtherComp :type "PrimitiveComponent Object Reference") (OtherBodyIndex :type Integer) (bFromSweep :type Boolean) (SweepResult :type "HitResult Structure (by ref)"))
  ;[1 1 1] Proche de la cachette
  (`SceneComponent.SetVisibility` (`self.Text`) true false))

(event `self.Collision.OnComponentEndOverlap`
  (params (OverlappedComponent :type "PrimitiveComponent Object Reference") (OtherActor :type "Actor Object Reference") (OtherComp :type "PrimitiveComponent Object Reference") (OtherBodyIndex :type Integer))
  ;[1 1 1] Proche de la cachette
  (`SceneComponent.SetVisibility` (`self.Text`) false false))

(event `InputAction|Action`
  (params (Key :type "Key Structure"))
  ;[1 1 1] Retour au personnage principal
  (:`Pressed`
    (bind _outactors (`GameplayStatics.GetAllActorsOfClass` "/Game/Personnage/BP_personnage.BP_personnage_C"))
    (for _array_element _outactors
      (`Controller.Possess` (`GameplayStatics.GetPlayerController` 0) _array_element)
      (`self.SetActorHiddenInGame` _array_element false)
      ;[1 1 1] Sound Barrel Out
      (`FMODAudioComponent.Play` (`self.SND_BarrelOut`)))))

(fn `UserConstructionScript`)