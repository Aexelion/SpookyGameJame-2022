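; Player character pawn with camera-relative movement, endurance-limited sprint, spring-arm pitch and look-back, and hiding in hideouts.
; The action input branches on a clothes check: throwing only plays a sound when an enemy is seen and in range, while hiding possesses an overlapping BP_cachette.
; Tick raises stress up to a maximum unless paused, but StressEffect is empty, the sound parameter update is disconnected and the clothes-count comparison is unwired.
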(event `InputAxis|MoveForward`
  (params (AxisValue :type "Float (single-precision)"))
  (bind (_returnvalue_roll _returnvalue_pitch _returnvalue_yaw) (`KismetMathLibrary.BreakRotator` (`self.GetControlRotation`)))
  ;[1 1 1] Déplacement
  (`self.AddMovementInput` (`KismetMathLibrary.GetForwardVector` (`KismetMathLibrary.MakeRotator` 0.0 0.0 _returnvalue_yaw)) AxisValue))

(event `InputAxis|Sprint`
  (params (AxisValue :type "Float (single-precision)"))
  (bind _charactermovement (`self.CharacterMovement`))
  ;[1 1 1] Sprint
  (set `self.TrySprint` (!= AxisValue 0.0))
  (bind _endurence (`self.UpdateEndurance`))
  (if (`self.TrySprint`)
    (bind _cansprint (`self.CanSprint` _endurence))
    (if _cansprint
      (set `CharacterMovementComponent.MaxWalkSpeed` 800.0 _charactermovement)
      (else
        (set `CharacterMovementComponent.MaxWalkSpeed` 450.0 _charactermovement :!label _label)))
    (else
      (goto _label))))

(event `InputAxis|MoveRight`
  (params (AxisValue :type "Float (single-precision)"))
  (bind (_returnvalue_roll _returnvalue_pitch _returnvalue_yaw) (`KismetMathLibrary.BreakRotator` (`self.GetControlRotation`)))
  ;[1 1 1] Déplacement
  (`self.AddMovementInput` (`KismetMathLibrary.GetRightVector` (`KismetMathLibrary.MakeRotator` 0.0 0.0 _returnvalue_yaw)) AxisValue))

(event `InputAction|Action`
  (params (Key :type "Key Structure"))
  ;[1 1 1] Action
  (:`Pressed`
    (if (`self.HaveAllClothes` (`self.nbClothes`))
      (`self.ThrowingCloth`)
      (else
        (`self.HideAction`)))))

(event `InputAxis|Turn`
  (params (AxisValue :type "Float (single-precision)"))
  ;[1 1 1] Mouvement Caméra Libre
  (`self.AddControllerYawInput` AxisValue))

(event `self.ReceiveTick`
  (params (DeltaSeconds :type "Float (single-precision)"))
  ;[1 1 1] Stress
  (set `self.DeltaTime` DeltaSeconds)
  (if (not (`self.GamePause`))
    (bind _stresslevel (`self.UpdateStress`))
    (`self.StressEffect` _stresslevel)))

(event `InputAxis|LookUp`
  (params (AxisValue :type "Float (single-precision)"))
  (bind _returnvalue (* AxisValue -1.0))
  (bind (_returnvalue_roll _returnvalue_pitch) (`KismetMathLibrary.BreakRotator` (`SceneComponent.K2_GetComponentRotation` (`self.SpringArm`))))
  (bind _returnvalue_2 (+ _returnvalue_pitch _returnvalue))
  ;[1 1 1] Mouvement Caméra Libre
  (if (and (> _returnvalue_2 -89.0) (< _returnvalue_2 89.0))
    (`SceneComponent.K2_AddRelativeRotation` (`self.SpringArm`) (`KismetMathLibrary.MakeRotator` 0.0 _returnvalue) false false)))

(event `InputAxis|LookBack`
  (params (AxisValue :type "Float (single-precision)"))
  (bind _springarm (`self.SpringArm`))
  (bind (_returnvalue_roll _returnvalue_pitch) (`KismetMathLibrary.BreakRotator` (`SpringArmComponent.GetTargetRotation` _springarm)))
  ;[1 1 1] Mouvement Caméra Libre
  (`SceneComponent.K2_SetRelativeRotation` _springarm (`KismetMathLibrary.MakeRotator` _returnvalue_roll _returnvalue_pitch (* AxisValue 180.0)) false false))

(fn `CanSprint`
  (params (Endurence :type "Float (double-precision)"))
  (returns (CanSprint :type Boolean))
  (return (> Endurence 0.0)))

(fn `ClothPickup`
  (set `self.nbClothes` (+ (`self.nbClothes`) 1)))

(fn `GoToHide`
  (bind _hideout (`self.Hideout`))
  (set `self.Hidden` true)
  (message `/Game/Personnage/BPI_hideout.Interact` _hideout self)
  (`Controller.Possess` (`GameplayStatics.GetPlayerController` 0) _hideout))

(fn `HideAction`
  (bind _hideoutinrange (`self.IsHideoutInRange`))
  (if _hideoutinrange
    (`self.GoToHide`)))

(fn `IsHideoutInRange`
  (returns (HideoutInRange :type Boolean) (HideoutPosition :type "Vector Structure"))
  (locals (Actor :type "Actor Object Reference"))
  (set `self.HideoutInRange` false)
  (for _array_element (`self.GetOverlappingActors` null)
    (if (`KismetSystemLibrary.DoesImplementInterface` _array_element "/Game/Personnage/BPI_hideout.BPI_hideout_C")
      (bind _output_get (set `self.HideoutInRange` true))
      (set `self.SavedHideoutPosition` (`self.K2_GetActorLocation` _array_element))
      (bind _asbp_cachette (cast `/Game/Personnage/Cachette/BP_cachette` _array_element))
      (set `self.Hideout` _asbp_cachette)))
  (return _output_get (0.0 0.0 0.0)))

(fn `StressEffect`
  (params (StressLevel :type "Float (double-precision)")))

(fn `ThrowingCloth`
  (if (`self.EnnemiInSight`)
    (if (`self.EnnemiInRange`)
      (`FMODBlueprintStatics.PlayEvent2D` "/Game/FMOD/Events/ENY/ENY_PutCloth.ENY_PutCloth"))))

(fn `UpdateEndurance`
  (returns (Endurence :type "Float (double-precision)"))
  (bind _maxendurance (`self.MaxEndurance`))
  (if (`self.TrySprint`)
    ;[1 1 1] Perte endurance
    (bind _output_get (set `self.Endurance` (+ (`self.Endurance`) (* (`self.DeltaTime`) -1.0))))
    (if (<= _output_get 0.0)
      (set `self.Endurance` 0.0))
    (else
      ;[1 1 1] Regain endurance
      (bind _output_get_2 (set `self.Endurance` (+ (`self.Endurance`) (* (`self.DeltaTime`) 3.0))))
      (if (> _output_get_2 _maxendurance)
        (set `self.Endurance` _maxendurance))))
  (return (`self.Endurance`)))

(fn `UpdateStress`
  (returns (StressLevel :type "Float (double-precision)"))
  (if (< (`self.StressLevel`) (`self.MaxStressLevel`))
    (bind _output_get (set `self.StressLevel` (+ (`self.StressLevel`) (`self.DeltaTime`))))
    (return _output_get)))

(fn `UserConstructionScript`)