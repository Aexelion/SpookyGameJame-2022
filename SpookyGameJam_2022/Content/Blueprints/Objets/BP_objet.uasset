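; BP_objet is a collectable clothing item that adds one to the player's clothes count when picked up.
; Entering or leaving ColectRangeBox toggles CanCollect on any BP_personnage tagged Player.
; The Collectable event, which nothing in this Blueprint calls, increments NbClothes once, guarded by HasBeenCollected.
; It then hides the static mesh and disables its collision instead of destroying the actor.
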(event `/Game/Personnage/BPI_collectable.Collectable`
  (params (Player :type "/Game/Personnage/BP_personnage Object Reference"))
  (bind _staticmesh (`self.StaticMesh`))
  ;[1 1 1] Interaction
  (if (not (`self.HasBeenCollected`))
    (set `/Game/Personnage/BP_personnage.NbClothes` (+ (`/Game/Personnage/BP_personnage.NbClothes` Player) 1) Player)
    (set `self.HasBeenCollected` true)
    (`SceneComponent.SetVisibility` _staticmesh false false)
    (`PrimitiveComponent.SetCollisionEnabled` _staticmesh "NoCollision")))

(event `self.ColectRangeBox.OnComponentBeginOverlap`
  (params (OverlappedComponent :type "PrimitiveComponent Object Reference") (OtherActor :type "Actor Object Reference") (OtherComp :type "PrimitiveComponent Object Reference") (OtherBodyIndex :type Integer) (bFromSweep :type Boolean) (SweepResult :type "HitResult Structure (by ref)"))
  ;[1 1 1] Proche du coffre
  (if (`self.ActorHasTag` OtherActor "Player")
    (bind _asbp_personnage (cast `/Game/Personnage/BP_personnage` OtherActor))
    (set `/Game/Personnage/BP_personnage.CanCollect` true _asbp_personnage)))

(event `self.ColectRangeBox.OnComponentEndOverlap`
  (params (OverlappedComponent :type "PrimitiveComponent Object Reference") (OtherActor :type "Actor Object Reference") (OtherComp :type "PrimitiveComponent Object Reference") (OtherBodyIndex :type Integer))
  ;[1 1 1] Proche du coffre
  (if (`self.ActorHasTag` OtherActor "Player")
    (bind _asbp_personnage (cast `/Game/Personnage/BP_personnage` OtherActor))
    (set `/Game/Personnage/BP_personnage.CanCollect` false _asbp_personnage)))

(fn `UserConstructionScript`)