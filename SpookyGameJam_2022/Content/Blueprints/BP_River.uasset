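; River actor that builds its shape along a spline and keeps its 3D river sound beside the player.
; The construction script adds a collision-enabled spline mesh component at each River spline point, matching locations and tangents toward the next point.
; On BeginPlay it caches the BP_personnage character, then a self-repeating delay loop moves SNDRiver3D to just above the closest spline point to the player, simulating sound along the whole river.
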(event `self.ReceiveBeginPlay`
  ;[1 1 1] Sound On River
  (bind _asbp_personnage (cast `/Game/Personnage/BP_personnage` (`GameplayStatics.GetPlayerCharacter` 0)))
  (set `self.CharacterReference` _asbp_personnage)
  (`self.MoveAudio`))

(event `MoveAudio`
  (bind (_returnvalue_x _returnvalue_y _returnvalue_z) (`KismetMathLibrary.BreakVector` (`SplineComponent.FindLocationClosestToWorldLocation` (`self.river`) (`self.K2_GetActorLocation` (`self.CharacterReference`)) "World")))
  ;[1 1 1] Sound On River
  (`SceneComponent.K2_SetWorldLocation` (`self.SND_River3D`) (`KismetMathLibrary.MakeVector` _returnvalue_x _returnvalue_y (+ _returnvalue_z 50.0)) false false)
  (`KismetSystemLibrary.Delay` 0.05)
  (`self.MoveAudio`))

(fn `UserConstructionScript`
  (bind _river (`self.river`))
  (bind _river_2 (`self.river`))
  (for _index (range (`SplineComponent.GetNumberOfSplinePoints` (`self.river`)))
    (bind _returnvalue (`AddComponent|NODE_AddSplineMeshComponent-1`))
    (`SplineMeshComponent.SetForwardAxis` _returnvalue "X" true)
    (`PrimitiveComponent.SetCollisionEnabled` _returnvalue "QueryAndPhysics")
    (bind _returnvalue_2 (+ _index 1))
    (`SplineMeshComponent.SetStartAndEnd` _returnvalue (`SplineComponent.GetLocationAtSplinePoint` _river_2 _index "Local") (`SplineComponent.GetTangentAtSplinePoint` _river_2 _index "Local") (`SplineComponent.GetLocationAtSplinePoint` _river _returnvalue_2 "Local") (`SplineComponent.GetTangentAtSplinePoint` _river _returnvalue_2 "Local") true)))