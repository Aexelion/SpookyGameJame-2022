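; SND_RiverSpline is an audio actor that makes river sound follow the player along a spline.
; On BeginPlay it casts the player character to BP_personnage, stores it and starts MoveAudio.
; MoveAudio moves the SNDRiver3D sound and an Arrow to the spline point closest to the player, raised slightly in Z.
; It then calls itself again after a short delay, forming a polling loop instead of using Tick.
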(event `self.ReceiveBeginPlay`
  (bind _asbp_personnage (cast `/Game/Personnage/BP_personnage` (`GameplayStatics.GetPlayerCharacter` 0)))
  (set `self.ChracterReference` _asbp_personnage)
  (`self.MoveAudio`))

(event `MoveAudio`
  (bind (_returnvalue_x _returnvalue_y _returnvalue_z) (`KismetMathLibrary.BreakVector` (`SplineComponent.FindLocationClosestToWorldLocation` (`self.SND_Spline`) (`self.K2_GetActorLocation` (`self.ChracterReference`)) "World")))
  (`SceneComponent.K2_SetWorldLocation` (`self.SND_River3D`) (`KismetMathLibrary.MakeVector` _returnvalue_x _returnvalue_y (+ _returnvalue_z 50.0)) false false)
  (`SceneComponent.K2_SetWorldLocation` (`self.Arrow`) (`KismetMathLibrary.MakeVector` _returnvalue_x _returnvalue_y (+ _returnvalue_z 50.0)) false false)
  (`KismetSystemLibrary.Delay` 0.05)
  (`self.MoveAudio`))

(fn `UserConstructionScript`)