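; BP_Road is an environment road Blueprint that builds spline mesh components from its Road spline.
; The construction script divides spline length by Length to set the loop count, adding an X-forward mesh component with query and physics collision each pass.
; Every component spans spline points 0 to 1 because the loop index is unused, so segments overlap.
; Only the start tangent is clamped to Length.
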(fn `UserConstructionScript`
  (bind _returnvalue (+ 0 1))
  (bind _road (`self.Road`))
  (bind _road_2 (`self.Road`))
  (for _index (range (+ (`KismetMathLibrary.FTrunc` (/ (`SplineComponent.GetSplineLength` (`self.Road`)) (`self.Length`))) 1))
    (bind _returnvalue_2 (`AddComponent|NODE_AddSplineMeshComponent-1`))
    (`SplineMeshComponent.SetForwardAxis` _returnvalue_2 "X" true)
    (`PrimitiveComponent.SetCollisionEnabled` _returnvalue_2 "QueryAndPhysics")
    (`SplineMeshComponent.SetStartAndEnd` _returnvalue_2 (`SplineComponent.GetLocationAtSplinePoint` _road_2 0 "Local") (`KismetMathLibrary.ClampVectorSize` (`SplineComponent.GetTangentAtSplinePoint` _road_2 0 "Local") 0.0 (`self.Length`)) (`SplineComponent.GetLocationAtSplinePoint` _road _returnvalue "Local") (`SplineComponent.GetTangentAtSplinePoint` _road _returnvalue "Local") true)))