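; BP_River is an environment Blueprint that builds a river along a spline.
; The Construction Script loops over every point of the River spline, adding an X-forward spline mesh with query and physics collision for each.
; Each segment takes its local position and tangent from that point and the next; the loop also runs on the last point.
; The event graph holds no gameplay logic.
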(fn `UserConstructionScript`
  (bind _river (`self.river`))
  (bind _river_2 (`self.river`))
  (for _index (range (`SplineComponent.GetNumberOfSplinePoints` (`self.river`)))
    (bind _returnvalue (`AddComponent|NODE_AddSplineMeshComponent-1`))
    (`SplineMeshComponent.SetForwardAxis` _returnvalue "X" true)
    (`PrimitiveComponent.SetCollisionEnabled` _returnvalue "QueryAndPhysics")
    (bind _returnvalue_2 (+ _index 1))
    (`SplineMeshComponent.SetStartAndEnd` _returnvalue (`SplineComponent.GetLocationAtSplinePoint` _river_2 _index "Local") (`SplineComponent.GetTangentAtSplinePoint` _river_2 _index "Local") (`SplineComponent.GetLocationAtSplinePoint` _river _returnvalue_2 "Local") (`SplineComponent.GetTangentAtSplinePoint` _river _returnvalue_2 "Local") true)))