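; Enemy character that catches the player and changes appearance as it gains clothing.
; Interact increments NbCloth, and DressedUp swaps skeletal mesh and animation asset for three stages, the last two sharing a mesh.
; KillingBox overlap with a non-hidden BP_personnage sets the IsKillingPlayer Blackboard key and the player's CaughtByEnemy flag.
; It also plays an attached sound on BeginPlay and exposes a function to set walk speed.
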(event `self.ReceiveBeginPlay`
  (`GameplayStatics.SpawnSoundAttached` null (`self.Audio`) "None" (0.0 0.0 0.0) (struct) "KeepRelativeOffset" false 1.0 1.0 0.0 null null))

(event `/Game/Ennemi/BPI_interactible.Interact`
  (`self.UpdateNbCloth` (+ (`self.NbCloth`) 1)))

(event `self.ReceiveTick`
  (params (DeltaSeconds :type "Float (single-precision)")))

(event `self.KillingBox.OnComponentBeginOverlap`
  (params (OverlappedComponent :type "PrimitiveComponent Object Reference") (OtherActor :type "Actor Object Reference") (OtherComp :type "PrimitiveComponent Object Reference") (OtherBodyIndex :type Integer) (bFromSweep :type Boolean) (SweepResult :type "HitResult Structure (by ref)"))
  ;[1 1 1] Attraper le joueur
  (bind _asbp_personnage (cast `/Game/Personnage/BP_personnage` OtherActor))
  (if (not (`/Game/Personnage/BP_personnage.Hidden` _asbp_personnage))
    (`BlackboardComponent.SetValueAsBool` (`AIBlueprintHelperLibrary.GetBlackboard` null) (`self.IsKillingPlayer`) true)
    (set `/Game/Personnage/BP_personnage.CaughtByEnemy` true _asbp_personnage)))

(fn `DressedUp`
  (params (NbCloth :type Integer))
  ;[1 1 1] Changement d'apparence
  (switch `int` NbCloth
    (:`0`
      (`SkinnedMeshComponent.SetSkinnedAssetAndUpdate` (`self.Mesh`) "/Game/Ennemi/Mechant01/SM_Mechant_01.SM_Mechant_01" false)
      (`SkeletalMeshComponent.SetAnimation` (`self.Mesh`) "/Game/Ennemi/BS_ennemi_01.BS_ennemi_01"))
    (:`1`
      (`SkinnedMeshComponent.SetSkinnedAssetAndUpdate` (`self.Mesh`) "/Game/Ennemi/Mechant02/SM_Mechant_02.SM_Mechant_02" false)
      (`SkeletalMeshComponent.SetAnimation` (`self.Mesh`) "/Game/Ennemi/BS_ennemi_02.BS_ennemi_02"))
    (:`2`
      (`SkinnedMeshComponent.SetSkinnedAssetAndUpdate` (`self.Mesh`) "/Game/Ennemi/Mechant02/SM_Mechant_02.SM_Mechant_02" false)
      (`SkeletalMeshComponent.SetAnimation` (`self.Mesh`) "/Game/Ennemi/BS_ennemi_03.BS_ennemi_03"))))

(fn `Update Walk Speed`
  (params (`New Walk Speed` :type "Float (double-precision)"))
  (set `CharacterMovementComponent.MaxWalkSpeed` `New Walk Speed` (`self.CharacterMovement`)))

(fn `UpdateNbCloth`
  (params (NewNbCloth :type Integer))
  (bind _output_get (set `self.NbCloth` NewNbCloth))
  (`self.DressedUp` _output_get))

(fn `UserConstructionScript`)